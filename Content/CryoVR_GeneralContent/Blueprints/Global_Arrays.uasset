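; Global_Arrays is a Blueprint that holds step-progress state, apparently for a step-based CryoVR procedure.
; SetStatus and GetStatus write and read the current step in Status.
; MovetoNextStep advances Status to the given next step only when it matches the supplied current step, so out-of-order calls change nothing.
; RecordCurrentStep separately appends each step it is given to StepRecord, a comma-delimited string log.
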(fn SetStatus
  (params (step :type Integer))
  (Variables|Default|SetStatus step))

(fn GetStatus
  (return (Variables|Default|GetStatus)))

(fn RecordCurrentStep
  (params (CurrentStep :type String))
  (Variables|Default|SetStepRecord (Utilities|String|Append (Variables|Default|GetStepRecord) CurrentStep ",")))

(fn MovetoNextStep
  (params (CurrentStep :type Integer) (NextStep :type Integer))
  (bind _step (CallFunction|GetStatus))
  (if (== _step CurrentStep)
    (CallFunction|SetStatus NextStep)))