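; Blueprint function library for CryoVR that supports grading and reporting of a step-based training module.
; It filters repeated steps logged within ten seconds into a comma-separated string and parses grading responses into score, result text and missing steps.
; Scores, missing-step descriptions and per-user step arrays live in the Global_Arrays game instance.
; Helpers also build Windows (ORCID) or Android (random-code) JSON payloads, generate digit codes and spawn 2D sound.
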(fn CheckDuplicateSteps
  (params (Steps :type Array%20of%20Integers) (Time :type Array%20of%20Floats%20%28single-precision%29))
  (bind _output_get (LocalVariables|SettempString ""))
  (LocalVariables|SettempString (Utilities|String|Append (Utilities|String|Append _output_get (Utilities|String|ToString(Integer) (Utilities|Array|Get(acopy) Steps))) ","))
  (for (_ _array_index) Steps
    ;[1 1 1] Skip first element
    (if (not (== _array_index 0))
      (if (not (and (== (Utilities|Array|Get(acopy) Steps _array_index) (Utilities|Array|Get(acopy) Steps (- _array_index 1))) (<= (- (Utilities|Array|Get(acopy) Time _array_index) (Utilities|Array|Get(acopy) Time (- _array_index 1))) 1e+01)))
        (LocalVariables|SettempString (Utilities|String|Append (Utilities|String|Append (LocalVariables|GettempString) (Utilities|String|ToString(Integer) (Utilities|Array|Get(acopy) Steps _array_index))) ",")))))
  (return (LocalVariables|GettempString)))

(fn RecordMissingStepstoGlobalArray
  (params (MissingStepsArray :type Array%20of%20Strings))
  (for _array_element MissingStepsArray
    (bind _asglobal_arrays (Utilities|Casting|CastToGlobal_Arrays (Game|GetGameInstance)))
    (Utilities|Array|Add (Variables|/Game/CryoVR_GeneralContent/Blueprints/Global_Arrays.Global_Arrays_C|GetMissing_Steps _asglobal_arrays) (.Value (Utilities|Map|Find (Variables|/Game/CryoVR_GeneralContent/Blueprints/Global_Arrays.Global_Arrays_C|GetIndex&Descriptions _asglobal_arrays) (Math|Conversions|ToInteger(Byte) (.RightS (Utilities|String|Split _array_element "Step")))))))
  (return))

(fn SpawnSound
  (bind _returnvalue (Audio|SpawnSound2D 0 0 1.0 1.0 0.0 0 false false))
  (return _returnvalue))

(fn GetResultandRecordScore
  (params (response :type Va%20Rest%20Json%20Object%20Object%20Reference) (time :type Float%20%28single-precision%29))
  (bind _returnvalue (Class|VaRestJsonObject|GetIntegerField response "score"))
  (bind _returnvalue_2 (Utilities|String|ToString(Integer) _returnvalue))
  ;[1 1 1] Get result string
  (bind _output_get (LocalVariables|SetResultString "Final Grade : "))
  ;[1 1 1] Record final score
  (bind _asglobal_arrays (Utilities|Casting|CastToGlobal_Arrays (Game|GetGameInstance)))
  (bind _output_get_2 (Variables|/Game/CryoVR_GeneralContent/Blueprints/Global_Arrays.Global_Arrays_C|SetScore _asglobal_arrays _returnvalue_2))
  (return (Utilities|String|Append (Utilities|String|Append (Utilities|String|Append _output_get _returnvalue_2) " / 100 ---------------- ") (Class|KismetStringLibrary|TimeSecondstoString time)) (Math|Conversions|ToInteger(Byte) _output_get_2) (Class|VaRestJsonObject|GetStringArrayField response "missStepstext")))

(fn MakeJsonforWindows
  (bind _asglobal_arrays (Utilities|Casting|CastToGlobal_Arrays (Game|GetGameInstance)))
  (return (Utilities|Enum|NotEqual(Enum) (Variables|/Game/CryoVR_GeneralContent/Blueprints/Global_Arrays.Global_Arrays_C|GetORCID _asglobal_arrays) "") (|MakeJson (Variables|/Game/CryoVR_GeneralContent/Blueprints/Global_Arrays.Global_Arrays_C|GetORCID _asglobal_arrays) (Variables|/Game/CryoVR_GeneralContent/Blueprints/Global_Arrays.Global_Arrays_C|GetModule _asglobal_arrays) (Variables|/Game/CryoVR_GeneralContent/Blueprints/Global_Arrays.Global_Arrays_C|GetVersion _asglobal_arrays) (Variables|/Game/CryoVR_GeneralContent/Blueprints/Global_Arrays.Global_Arrays_C|GetScore _asglobal_arrays))))

(fn MakeJsonforAndroid
  (params (code :type String))
  (bind _asglobal_arrays (Utilities|Casting|CastToGlobal_Arrays (Game|GetGameInstance)))
  (return (|MakeJson code (Variables|/Game/CryoVR_GeneralContent/Blueprints/Global_Arrays.Global_Arrays_C|GetModule _asglobal_arrays) (Variables|/Game/CryoVR_GeneralContent/Blueprints/Global_Arrays.Global_Arrays_C|GetVersion _asglobal_arrays) (Variables|/Game/CryoVR_GeneralContent/Blueprints/Global_Arrays.Global_Arrays_C|GetScore _asglobal_arrays))))

(fn GenerateRandomCode
  (params (digitNumber :type Integer))
  (for _index (range 1 digitNumber)
    (LocalVariables|Setcode (Utilities|String|Append (LocalVariables|Getcode) (Utilities|String|ToString(Integer) (Math|Random|RandomIntegerinRange 0 9)))))
  (return (LocalVariables|Getcode)))

(fn ClearStepArrays
  (bind _asglobal_arrays (Utilities|Casting|CastToGlobal_Arrays (Game|GetGameInstance)))
  (Utilities|Array|Clear (Variables|/Game/CryoVR_GeneralContent/Blueprints/Global_Arrays.Global_Arrays_C|GetUser_Description_Array _asglobal_arrays))
  (Utilities|Array|Clear (Variables|/Game/CryoVR_GeneralContent/Blueprints/Global_Arrays.Global_Arrays_C|GetUser_Time_Array _asglobal_arrays))
  (Utilities|Array|Clear (Variables|/Game/CryoVR_GeneralContent/Blueprints/Global_Arrays.Global_Arrays_C|GetUser_Index_Array _asglobal_arrays))
  (Utilities|Array|Clear (Variables|/Game/CryoVR_GeneralContent/Blueprints/Global_Arrays.Global_Arrays_C|GetCorrect_Answers _asglobal_arrays))
  (Utilities|Array|Clear (Variables|/Game/CryoVR_GeneralContent/Blueprints/Global_Arrays.Global_Arrays_C|GetMissing_Steps _asglobal_arrays))
  (return))